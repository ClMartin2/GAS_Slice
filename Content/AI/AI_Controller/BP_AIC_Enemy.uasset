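; AI controller for enemy pawns that tracks what its perception sees and fires the pawn's gun.
; On possess it waits one tick, then caches the Enemy pawn and its SMCGun component.
; Perception updates store the sensed actor and whether it is currently seen, while a Shoot event fires the gun after a FireRate delay.
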(event `self.ReceivePossess`
  (params (PossessedPawn :type "Pawn Object Reference"))
  (`KismetSystemLibrary.DelayUntilNextTick`)
  (bind _asenemy (cast `Enemy` PossessedPawn))
  (bind _output_get (set `self.Enemy` _asenemy))
  (set `self.SMCGun` (`Enemy.SMCGun` _output_get)))

(event `self.AIPerception.OnTargetPerceptionUpdated`
  (params (Actor :type "Actor Object Reference") (Stimulus :type "AIStimulus Structure"))
  (set `self.ActorSeen` Actor)
  (set `self.SeeEnemy` (`.bSuccessfullySensed` (break `AIStimulus` Stimulus))))

(event `Shoot`
  (`KismetSystemLibrary.Delay` (`self.FireRate`))
  (`SMC_Gun.Shoot` (`self.SMCGun`)))

(fn `UserConstructionScript`)