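; Player character Blueprint that casts a fire spell through the Gameplay Ability System.
; BeginPlay grants GA_FireSpell, stores its handle and applies the GE_RegenMana effect to itself.
; A debug F key activates the stored ability, and Tick prints the base Mana value from BasicAttributeSet.
; GetTransformSpawnSpell exposes the world transform of the SpawnSpellPosition component as a spell spawn point.
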(event EventBeginPlay
  (|CallParentFunction)
  (bind _returnvalue (GameplayAbilities|GiveAbility (Variables|Default|GetAbilitySystemComponent) "/Game/Blueprints/GameplayAbilities/GA_FireSpell.GA_FireSpell_C" 0 -1))
  (Variables|Default|SetNewVar _returnvalue)
  (GameplayEffects|ApplyGameplayEffectToSelf :self (Variables|Default|GetAbilitySystemComponent) :GameplayEffectClass "/Game/Blueprints/GameplayEffects/GE_RegenMana.GE_RegenMana_C"))

(event EventTick
  (params (DeltaSeconds :type Float%20%28single-precision%29))
  (bind _returnvalue (GameplayAttributes|GetAttributeSet (Variables|Default|GetAbilitySystemComponent) "/Script/GAS_Slice.BasicAttributeSet"))
  (Development|PrintString (Utilities|String|ToString(Float) (.basevalue (Variables|/Script/GAS_Slice.BasicAttributeSet|GetMana _returnvalue))) true true "(R=0.000000,G=0.660000,B=1.000000,A=1.000000)" 0.0))

(event Input|KeyboardEvents|DebugKeyF
  (params (Key :type Key%20Structure :default "None") (ActionValue :type Input%20Action%20Value%20Structure))
  (:Pressed
    (bind _returnvalue (Class|AbilitySystemComponent|TryActivateAbility (Variables|Default|GetAbilitySystemComponent) (Variables|Default|GetNewVar) true))
    (if _returnvalue
      _)))

(fn ConstructionScript)

(fn GetTransformSpawnSpell
  (return (Transformation|GetWorldTransform (Variables|Default|GetSpawnSpellPosition))))