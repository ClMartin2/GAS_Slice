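; Player controller for a first-person knife-throwing spellcaster, building the HUD and restarting the game at zero health.
; Grants GAS abilities by input index, with mana regen, and switches between five spells.
; Extends parent knife and landing events with timelines that check knife distance and, after a delay, step down push force and speed.
; Tick scales FOV with speed; gameplay-tag listeners and shield checks drive shield HUD animations.
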(event `self.ReceiveBeginPlay`
  ;[0 0 0] Begin play
  (`parent.ReceiveBeginPlay`)
  (bind _asbp_player_character (cast `/Game/Blueprints/BP_PlayerCharacter` (`GameplayStatics.GetPlayerCharacter` 0)))
  (set `self.BP_PlayerCharacter` _asbp_player_character)
  (`self.GiveAbility`)
  (bind _returnvalue (`|CreateWidget` "/Game/UI/WG_Hud.WG_Hud_C" self))
  (set `self.WG_Hud` _returnvalue)
  (set `/Game/UI/WG_Hud.BP_PlayerCharacter` (`self.BP_PlayerCharacter`) (`self.WG_Hud`))
  (`UserWidget.AddToViewport` (`self.WG_Hud`) 0)
  (`AbilityAsync_WaitGameplayTagAdded.WaitGameplayTagAddToActor` (`self.BP_PlayerCharacter`) (struct :`TagName` "Spell.Shield")
    (:`then`
      (`AbilityAsync_WaitGameplayTagRemoved.WaitGameplayTagRemoveFromActor` (`self.BP_PlayerCharacter`) (struct :`TagName` "Spell.Shield")
        (:`then`
          (set `self.StartFOV` (`CameraComponent.FieldOfView` (`GAS_SliceCharacter.FirstPersonCameraComponent` (`self.BP_PlayerCharacter`)))))
        (:`Removed`
          (if (not (`self.AlredayRemoveShieldAnimation`))
            (`/Game/UI/WG_Hud.PlayAnimationRemoveShield` (`self.WG_Hud`))))))
    (:`Added`
      (`/Game/UI/WG_Hud.PlayAnimationGainShield` (`self.WG_Hud`))
      (`self.ResetDoOnceRemoveShield`)
      (set `self.AlredayRemoveShieldAnimation` false))))

(event `self.ThrowKnife`
  ;[0 0 0] Throw knife
  (`parent.ThrowKnife`)
  (`TimelineComponent.PlayFromStart` (`self.TimelineUpdateCheckDistance`)))

(event `self.ResetKnife`
  ;[0 0 0] Reset Knife
  (`parent.ResetKnife`)
  (`TimelineComponent.Stop` (`self.TimelineUpdateCheckDistance`)))

(event `self.PullKnife`
  ;[0 0 0] Pull Knife
  (`parent.PullKnife`)
  (`self.StartReducingValue` (`self.CounterToStartRemovingActualForce`) (`self.CounterToRemoveForce`) (`self.TimelineReduceForce`))
  (`TimelineComponent.Stop` (`self.TimelineReduceSpeedWalk`))
  (set `self.AlreadyStartDecreaseSpeedValue` false))

(event `self.OnLandedCharacter`
  ;[0 0 0] On Landed Character
  (`parent.OnLandedCharacter`)
  (if (not (`self.AlreadyStartDecreaseSpeedValue`))
    (set `self.AlreadyStartDecreaseSpeedValue` true)
    (`self.StartReducingValue` (`self.CounterToStartRemovingSpeed`) (`self.CounterToRemoveSpeed`) (`self.TimelineReduceSpeedWalk`))))

(event `self.ReceiveTick`
  (params (DeltaSeconds :type "Float (single-precision)"))
  ;[0 0 0] Tick
  (`parent.ReceiveTick` DeltaSeconds)
  ;; Set FOV
  (`self.SetFOV`)
  ;;[0.149 0.149 0.149 0.502] Death
  (bind _death (`self.CheackDeath`))
  (if _death
    (`self.Death`)
    (else
      ;;[0.149 0.149 0.149 0.502] Check to Remove shield
      (bind _returnvalue (`AbilitySystemComponent.GetAttributeSet` (`AbilitySystemBlueprintLibrary.GetAbilitySystemComponent` (`self.BP_PlayerCharacter`)) "/Script/GAS_Slice.BasicAttributeSet"))
      (bind (_shield_basevalue _shield_currentvalue) (break `GameplayAttributeData` (`BasicAttributeSet.Shield` _returnvalue)))
      (if (<= _shield_currentvalue 0.0)
        (`/Engine/EditorBlueprintResources/StandardMacros.DoOnce` true :!label _label
          (:`Completed`
            (`/Game/UI/WG_Hud.PlayAnimationRemoveShield` (`self.WG_Hud`))
            (set `self.AlredayRemoveShieldAnimation` true)))))))

(event `ResetDoOnceRemoveShield`
  ;[0 0 0] Tick
  ;;[0.149 0.149 0.149 0.502] Check to Remove shield
  (goto _label :!via `Reset`))

(event `EnhancedInput|/Game/Inputs/Actions/Spells/IA_SwitchSpells1`
  (params (ActionValue :type Boolean) (ElapsedSeconds :type "Float (double-precision)") (TriggeredSeconds :type "Float (double-precision)") (InputAction :type "InputAction Object Reference" :default "/Game/Inputs/Actions/Spells/IA_SwitchSpells1.IA_SwitchSpells1"))
  ; Set Current Ability
  (:`Triggered`
    (`self.SwitchSpells` "NewEnumerator0")))

(event `EnhancedInput|/Game/Inputs/Actions/Spells/IA_SwitchSpells4`
  (params (ActionValue :type Boolean) (ElapsedSeconds :type "Float (double-precision)") (TriggeredSeconds :type "Float (double-precision)") (InputAction :type "InputAction Object Reference" :default "/Game/Inputs/Actions/Spells/IA_SwitchSpells4.IA_SwitchSpells4"))
  ; Set Current Ability
  (:`Triggered`
    (`self.SwitchSpells` "NewEnumerator3")))

(event `EnhancedInput|/Game/Inputs/Actions/Spells/IA_SwitchSpells2`
  (params (ActionValue :type Boolean) (ElapsedSeconds :type "Float (double-precision)") (TriggeredSeconds :type "Float (double-precision)") (InputAction :type "InputAction Object Reference" :default "/Game/Inputs/Actions/Spells/IA_SwitchSpells2.IA_SwitchSpells2"))
  ; Set Current Ability
  (:`Triggered`
    (`self.SwitchSpells` "NewEnumerator1")))

(event `EnhancedInput|/Game/Inputs/Actions/Spells/IA_SwitchSpells5`
  (params (ActionValue :type Boolean) (ElapsedSeconds :type "Float (double-precision)") (TriggeredSeconds :type "Float (double-precision)") (InputAction :type "InputAction Object Reference" :default "/Game/Inputs/Actions/Spells/IA_SwitchSpells5.IA_SwitchSpells5"))
  ; Set Current Ability
  (:`Triggered`
    (`self.SwitchSpells` "NewEnumerator4")))

(event `EnhancedInput|/Game/Inputs/Actions/Spells/IA_SwitchSpells3`
  (params (ActionValue :type Boolean) (ElapsedSeconds :type "Float (double-precision)") (TriggeredSeconds :type "Float (double-precision)") (InputAction :type "InputAction Object Reference" :default "/Game/Inputs/Actions/Spells/IA_SwitchSpells3.IA_SwitchSpells3"))
  ; Set Current Ability
  (:`Triggered`
    (`self.SwitchSpells` "NewEnumerator2")))

(event `EnhancedInput|/Game/Inputs/Actions/Spells/IA_UseSpells`
  (params (ActionValue :type Boolean) (ElapsedSeconds :type "Float (double-precision)") (TriggeredSeconds :type "Float (double-precision)") (InputAction :type "InputAction Object Reference" :default "/Game/Inputs/Actions/Spells/IA_UseSpells.IA_UseSpells"))
  (:`Triggered`
    (`AbilitySystemComponent.PressInputID` (`self.AbilitySystemComponent`) (`KismetMathLibrary.Conv_ByteToInt` (`self.CurrentAbility`)))))

(fn `CheackDeath`
  (returns (Death :type Boolean))
  (bind _returnvalue (`AbilitySystemComponent.GetAttributeSet` (`BaseCharacter.AbilitySystemComponent` (`self.BP_PlayerCharacter`)) "/Script/GAS_Slice.BasicAttributeSet"))
  (bind _health_basevalue (break `GameplayAttributeData` (`BasicAttributeSet.Health` _returnvalue)))
  (return (<= _health_basevalue 0.0)))

(fn `Death`
  (bind _asgame_mode (cast `GameMode` (`GameplayStatics.GetGameMode`)))
  (`GameMode.RestartGame` _asgame_mode))

(fn `DecreaseActualForce`
  (`self.SetActualPushForce` (* (`self.ReducePushForce`) -1.0)))

(fn `DecreaseActualSpeed`
  (`self.SetActualSpeed` (* (`self.ReduceSpeed`) -1.0)))

(fn `GiveAbility`
  (set `self.AbilitySystemComponent` (`AbilitySystemBlueprintLibrary.GetAbilitySystemComponent` (`GameplayStatics.GetPlayerCharacter` 0)))
  (for (_array_element _array_index) (`self.AbilityClass`)
    (`AbilitySystemComponent.K2_GiveAbility` (`self.AbilitySystemComponent`) _array_element 0 _array_index))
  (`AbilitySystemComponent.BP_ApplyGameplayEffectToSelf` :`self` (`self.AbilitySystemComponent`) :`GameplayEffectClass` "/Game/Blueprints/GameplayEffects/GE_RegenMana.GE_RegenMana_C"))

(fn `ReduceValue`
  (params (CounterToStartRemoving :type "Float (double-precision) (by ref)") (CounterToRemove :type "Float (double-precision) (by ref)") (TimeToStartRemoving :type "Float (double-precision)") (TimeToRemove :type "Float (double-precision)"))
  (returns (ReduceValue :type Boolean))
  (`|VariableSetRef` (`local.CounterToStartRemoving`) (+ (`local.CounterToStartRemoving`) (`GameplayStatics.GetWorldDeltaSeconds`)))
  (if (>= (`local.CounterToStartRemoving`) (`local.TimeToStartRemoving`))
    (`|VariableSetRef` (`local.CounterToRemove`) (+ (`local.CounterToRemove`) (`GameplayStatics.GetWorldDeltaSeconds`)))
    (if (>= (`local.CounterToRemove`) (`local.TimeToRemove`))
      (`|VariableSetRef` (`local.CounterToRemove`))
      (return true)
      (else
        (return false)))
    (else
      (return false))))

(fn `SetFOV`
  (`CameraComponent.SetFieldOfView` (`GAS_SliceCharacter.FirstPersonCameraComponent` (`self.PlayerCharacter`)) (`KismetMathLibrary.Lerp` (`self.StartFOV`) (`self.MaxFOV`) (/ (- (`self.CurrentSpeed`) (`self.MinCharacterSpeed`)) (- (`self.MaxCharacterSpeed`) (`self.MinCharacterSpeed`))))))

(fn `StartReducingValue`
  (params (CounterToStartRemovingActualForce :type "Float (double-precision) (by ref)") (CounterToRemoveForce :type "Float (double-precision) (by ref)") (TimeLine :type "TimelineComponent Object Reference"))
  (`TimelineComponent.PlayFromStart` TimeLine)
  (`|VariableSetRef` CounterToStartRemovingActualForce)
  (`|VariableSetRef` CounterToRemoveForce))

(fn `SwitchSpells`
  (params (Ability :type "/Game/Enumeration/E_Ability Enum" :default "NewEnumerator0"))
  (set `self.CurrentAbility` Ability)
  (`/Game/UI/WG_Hud.SwitchSpells` (`self.WG_Hud`) (`self.CurrentAbility`)))

(fn `UserConstructionScript`)