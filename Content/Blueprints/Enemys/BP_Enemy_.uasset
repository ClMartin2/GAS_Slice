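; BP_Enemy_ is an enemy character Blueprint that uses the Gameplay Ability System to drive its movement speed.
; On BeginPlay it sets max walk speed from the BasicAttributeSet's Speed, then a persistent attribute-change listener writes each new value to CharacterMovement.
; Tick prints debug readouts of walk speed, base Health and owned gameplay tags every frame.
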(event `self.OnBeginPlay`
  (`parent.OnBeginPlay`)
  (bind _returnvalue (`AbilitySystemComponent.GetAttributeSet` (`self.AbilitySystemComponent`) "/Script/GAS_Slice.BasicAttributeSet"))
  (bind (_speed_basevalue _speed_currentvalue) (break `GameplayAttributeData` (`BasicAttributeSet.Speed` _returnvalue)))
  (set `CharacterMovementComponent.MaxWalkSpeed` _speed_currentvalue (`self.CharacterMovement`))
  (bind (_asynctaskproxy _attribute _newvalue) (`AbilityAsync_WaitAttributeChanged.WaitForAttributeChanged` null (struct :`AttributeName` "Speed" :`Attribute` "/Script/GAS_Slice.BasicAttributeSet:Speed" :`AttributeOwner` "/Script/CoreUObject.Class'/Script/GAS_Slice.BasicAttributeSet'"))
    (:`Changed`
      (set `CharacterMovementComponent.MaxWalkSpeed` _newvalue (`self.CharacterMovement`)))))

(event `self.ReceiveTick`
  (params (DeltaSeconds :type "Float (single-precision)"))
  (bind _returnvalue_gameplaytags (break `GameplayTagContainer` (`BlueprintGameplayTagLibrary.GetOwnedGameplayTags` (`self.AbilitySystemComponent`))))
  (`KismetSystemLibrary.PrintString` (`KismetStringLibrary.Concat_StrStr` "Max WAlk Speed:" (`KismetStringLibrary.Conv_DoubleToString` (`CharacterMovementComponent.MaxWalkSpeed` (`self.CharacterMovement`)))) true true (struct :`G` 0.66 :`B` 1.0 :`A` 1.0) 0.0)
  (bind _returnvalue (`AbilitySystemComponent.GetAttributeSet` (`self.AbilitySystemComponent`) "/Script/GAS_Slice.BasicAttributeSet"))
  (bind _health_basevalue (break `GameplayAttributeData` (`BasicAttributeSet.Health` _returnvalue)))
  (`KismetSystemLibrary.PrintString` (`KismetStringLibrary.Concat_StrStr` "Enemy Health : " (`KismetStringLibrary.Conv_DoubleToString` _health_basevalue)) true true (struct :`G` 0.66 :`B` 1.0 :`A` 1.0) 0.0)
  (for _array_element _returnvalue_gameplaytags
    (`KismetSystemLibrary.PrintString` (`KismetStringLibrary.Conv_NameToString` (`BlueprintGameplayTagLibrary.GetTagName` _array_element)) true true (struct :`G` 0.66 :`B` 1.0 :`A` 1.0) 0.0)))

(fn `UserConstructionScript`)