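; GA_CastSpell is a gameplay ability that spawns a spell actor and charges mana for it.
; Activation is allowed only when the base Mana in BasicAttributeSet exceeds the absolute CostMana.
; After committing cost, avatars implementing BI_ThrowSpell supply the spawn transform for SpellClass, following an empty CastSpell hook.
; GE_UseMana then applies CostMana as a Spell.Mana SetByCaller magnitude, and the ability ends.
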(event `self.K2_ActivateAbility`
  (bind _returnvalue (`self.GetAvatarActorFromActorInfo`))
  (bind _returnvalue_2 (`self.K2_CommitAbilityCost` false))
  (if _returnvalue_2
    (if (`KismetSystemLibrary.DoesImplementInterface` _returnvalue "/Game/Interfaces/BI_ThrowSpell.BI_ThrowSpell_C")
      (`self.CastSpell`)
      (bind _transformtospawn (message `/Game/Interfaces/BI_ThrowSpell.GetTransformSpawnSpell` _returnvalue))
      (`|SpawnActorFromClass` (`self.SpellClass`) _transformtospawn "AdjustIfPossibleButAlwaysSpawn" "MultiplyWithRoot" (`self.GetAvatarActorFromActorInfo`) null)
      (bind _returnvalue_3 (`AbilitySystemBlueprintLibrary.AssignTagSetByCallerMagnitude` (`self.MakeOutgoingGameplayEffectSpec` "/Game/Blueprints/GameplayEffects/GE_UseMana.GE_UseMana_C") (struct :`TagName` "Spell.Mana") (`self.CostMana`)))
      (`self.K2_ApplyGameplayEffectSpecToOwner` _returnvalue_3)
      (`self.K2_EndAbility`)
      (else
        (`self.K2_EndAbility`)))
    (else
      (`self.K2_EndAbility`))))

(fn `CastSpell`)

(fn `K2_CanActivateAbility`
  (params (ActorInfo :type "GameplayAbilityActorInfo Structure") (Handle :type "GameplayAbilitySpecHandle Structure"))
  (returns (RelevantTags :type "GameplayTagContainer Structure") (ReturnValue :type Boolean))
  (bind _returnvalue (`AbilitySystemComponent.GetAttributeSet` (`AbilitySystemBlueprintLibrary.GetAbilitySystemComponent` ActorInfo_OwnerActor) "/Script/GAS_Slice.BasicAttributeSet"))
  (bind _mana_basevalue (break `GameplayAttributeData` (`BasicAttributeSet.Mana` _returnvalue)))
  (return (struct) (> _mana_basevalue (`KismetMathLibrary.Abs` (`self.CostMana`)))))