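; GA_ThrowProjectile is a Gameplay Ability that spawns a projectile from the avatar actor.
; On activation it commits only the ability cost, then asks the avatar for a spawn transform through the BI_ThrowSpell interface.
; It spawns ProjectileClass there with the avatar as owner, adjusting for collisions but always spawning.
; The ability ends immediately afterward, or without spawning if the cost or interface check fails.
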(event `self.K2_ActivateAbility`
  (bind _returnvalue (`self.GetAvatarActorFromActorInfo`))
  (bind _returnvalue_2 (`self.K2_CommitAbilityCost` false))
  (if _returnvalue_2
    (if (`KismetSystemLibrary.DoesImplementInterface` _returnvalue "/Game/Interfaces/BI_ThrowSpell.BI_ThrowSpell_C")
      (bind _transformtospawn (message `/Game/Interfaces/BI_ThrowSpell.GetTransformSpawnSpell` _returnvalue))
      (`|SpawnActorFromClass` (`self.ProjectileClass`) _transformtospawn "AdjustIfPossibleButAlwaysSpawn" "MultiplyWithRoot" _returnvalue null)
      (`self.K2_EndAbility`)
      (else
        (`self.K2_EndAbility`)))
    (else
      (`self.K2_EndAbility`))))