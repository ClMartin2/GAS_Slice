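; BP_FireSpell is a fire spell actor that extends a parent Blueprint, which handles the core begin-play and overlap logic.
; On sphere overlap it spawns its hit effect at the particle system's location, then calls the parent handler.
; BeginPlay only calls the parent, as the tinted shot shockwave effect is left disconnected and never runs.
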(event `self.ReceiveBeginPlay`
  ; Spawn Shot FX
  (`parent.ReceiveBeginPlay`))

(event `self.OnSphereBeginOverlap`
  (params (OverlappedComp :type "PrimitiveComponent Object Reference") (OtherActor :type "Actor Object Reference") (OtherComp :type "PrimitiveComponent Object Reference") (OtherBodyIndex :type Integer) (bFromSweep :type Boolean) (SweepResult :type "HitResult Structure (by ref)"))
  ; Spawn Hit FX
  (`GameplayStatics.SpawnEmitterAtLocation` (`self.hitFx`) (`SceneComponent.K2_GetComponentLocation` (`self.ParticleSystem`)))
  (`parent.OnSphereBeginOverlap` OverlappedComp OtherActor OtherComp OtherBodyIndex bFromSweep SweepResult))

(fn `UserConstructionScript`)