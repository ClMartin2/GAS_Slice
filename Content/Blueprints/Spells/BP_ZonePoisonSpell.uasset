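; BP_ZonePoisonSpell is a zone spell that shows a poison smoke effect when something overlaps its sphere.
; After the parent's overlap handling, each overlap spawns a new BP_FXPoisonSpell and stores it, overwriting the previous reference.
; It passes WorldSpaceSize to the FX component and drops the effect half that height below the zone's location.
; The Debug flag drives the effect's bounds drawing.
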(event `self.OnSphereBeginOverlap`
  (params (OverlappedComp :type "PrimitiveComponent Object Reference") (OtherActor :type "Actor Object Reference") (OtherComp :type "PrimitiveComponent Object Reference") (OtherBodyIndex :type Integer) (bFromSweep :type Boolean) (SweepResult :type "HitResult Structure (by ref)"))
  (bind (_worldspacesize_x _worldspacesize_y _worldspacesize_z) (`KismetMathLibrary.BreakVector` (`self.WorldSpaceSize`)))
  (`parent.OnSphereBeginOverlap` OverlappedComp OtherActor OtherComp OtherBodyIndex bFromSweep SweepResult)
  (bind _returnvalue (`|SpawnActorFromClass` "/Game/Blueprints/FX/BP_FXPoisonSpell.BP_FXPoisonSpell_C" (`KismetMathLibrary.MakeTransform` (0.0 0.0 0.0)) "Undefined" "MultiplyWithRoot" null null))
  (bind _output_get (set `self.BPFXPoisonSmoke` _returnvalue))
  (`NiagaraComponent.SetVariableVec3` (`/Game/Blueprints/FX/BP_FXPoisonSpell.FX` _output_get) "WorldSpaceSize" (`self.WorldSpaceSize`))
  (`self.K2_SetActorLocation` (`self.BPFXPoisonSmoke`) (- (`self.K2_GetActorLocation`) (`KismetMathLibrary.MakeVector` 0.0 0.0 (/ _worldspacesize_z 2.0))) false false)
  (`NiagaraComponent.SetVariableBool` (`/Game/Blueprints/FX/BP_FXPoisonSpell.FX` (`self.BPFXPoisonSmoke`)) "DrawBounds" (`KismetSystemLibrary.MakeLiteralBool` (`self.Debug`))))

(fn `UserConstructionScript`)